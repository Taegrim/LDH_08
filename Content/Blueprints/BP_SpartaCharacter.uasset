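; BP_SpartaCharacter is the character Blueprint that drives the HUD's vision-block overlay from active status effects.
; When status effects change, it sums the strength of every VisionRestriction effect into an alpha value.
; It then reaches WBP_HUD through the controller, cast to SpartaPlayerController, and sets the vision block alpha to that unclamped total.
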(event EventOnStatusEffectsChanged
  (params (StatusEffects :type Array%20of%20Active%20Status%20Effect%20Structures))
  (Variables|Default|SetAlpha 0.0)
  (for _array_element StatusEffects
    (if (Utilities|Enum|Equal(Enum) (.type _array_element) "VisionRestriction")
      (Variables|Default|SetAlpha (+ (Variables|Default|GetAlpha) (.strength _array_element)))))
  (bind _assparta_player_controller (Utilities|Casting|CastToSpartaPlayerController (Pawn|GetController)))
  (bind _aswbp_hud (Utilities|Casting|CastToWBP_HUD (Class|SpartaPlayerController|GetHUDWidget _assparta_player_controller)))
  (Default|SetVisionBlockAlpha _aswbp_hud (Variables|Default|GetAlpha)))

(fn ConstructionScript)